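; Example actor that shows the current in-game weekday number on a TextRender through weekly recurring time triggers.
; RegisterGameTimeEvent binds seven start times, Monday through Sunday, via addEveryWeekCircleEvents.
; Each callback runs identical logic, reading game time and writing its one-offset day of week as "{0} WeekDay" text.
; UnregisterGameTimeEvent cancels the binding, and no Tick polling is used.
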(event EventBeginPlay)

(event Collision|EventActorBeginOverlap
  (params (OtherActor :type Actor%20Object%20Reference)))

(event EventTick
  (params (DeltaSeconds :type Float%20%28single-precision%29)))

(event EventRegisterGameTimeEvent
  (bind _returnvalue (Class|XDTimeManagerFunctionLibrary|GetGameTime))
  (bind _returnvalue_2 (Class|XDGameTimeTypeFunctionLibrary|GetDayOfWeek _returnvalue))
  (bind _returnvalue_3 (+ _returnvalue_2 1))
  (bind _returnvalue_4 (Utilities|String|ToString(Byte) _returnvalue_3))
  (bind _returnvalue_5 (Utilities|Text|ToText(String) _returnvalue_4))
  (bind _result (Utilities|Text|FormatText "{0} WeekDay" _returnvalue_5))
  (|AddEveryWeekCircleEvents (Variables|Default|Get周一事件) (Variables|Default|Get周二事件) (Variables|Default|Get周三事件) (Variables|Default|Get周四事件) (Variables|Default|Get周五事件) (Variables|Default|Get周六事件) (Variables|Default|Get周日事件)
    (:事件[1]
      (Rendering|Components|TextRender|SetText (Variables|Default|GetTextRender) _result))
    (:事件[2]
      (Rendering|Components|TextRender|SetText (Variables|Default|GetTextRender) _result))
    (:事件[3]
      (Rendering|Components|TextRender|SetText (Variables|Default|GetTextRender) _result))
    (:事件[4]
      (Rendering|Components|TextRender|SetText (Variables|Default|GetTextRender) _result))
    (:事件[5]
      (Rendering|Components|TextRender|SetText (Variables|Default|GetTextRender) _result))
    (:事件[6]
      (Rendering|Components|TextRender|SetText (Variables|Default|GetTextRender) _result))
    (:事件[7]
      (Rendering|Components|TextRender|SetText (Variables|Default|GetTextRender) _result))))

(event EventUnregisterGameTimeEvent
  (bind _returnvalue (Class|XDTimeManagerFunctionLibrary|GetGameTime))
  (bind _returnvalue_2 (Class|XDGameTimeTypeFunctionLibrary|GetDayOfWeek _returnvalue))
  (bind _returnvalue_3 (+ _returnvalue_2 1))
  (bind _returnvalue_4 (Utilities|String|ToString(Byte) _returnvalue_3))
  (bind _returnvalue_5 (Utilities|Text|ToText(String) _returnvalue_4))
  (bind _result (Utilities|Text|FormatText "{0} WeekDay" _returnvalue_5))
  (|AddEveryWeekCircleEvents (Variables|Default|Get周一事件) (Variables|Default|Get周二事件) (Variables|Default|Get周三事件) (Variables|Default|Get周四事件) (Variables|Default|Get周五事件) (Variables|Default|Get周六事件) (Variables|Default|Get周日事件)) ; enters at 取消时间事件绑定
)

(fn ConstructionScript)